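; GA_Event_Damage is an event-activated test gameplay ability that reacts to damage events.
; When the owning actor is the event's instigator, it applies the GE_Test_LifeSteal effect to itself.
; It also looks up a DamageGameplayContext fragment in the effect context without acting on the result, then ends.
; Disconnected debug nodes would print magnitude and critical hit or fire a test GameplayCue.
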(event `self.K2_ActivateAbilityFromEvent`
  (params (EventData :type "GameplayEventData Structure (by ref)"))
  (bind (_eventtag _instigator _target _optionalobject _optionalobject2 _contexthandle _instigatortags _targettags _eventmagnitude) (break `GameplayEventData` EventData))
  (if (== _instigator (`self.GetOwningActorFromActorInfo`))
    (`self.BP_ApplyGameplayEffectToOwner` "/Game/FinalFantasyXI/AbilitySystem/Test/GE_Test_LifeSteal.GE_Test_LifeSteal_C"))
  (bind _value (`BlueprintInstancedStructLibrary.GetInstancedStructValue` (`CrimAbilitySystemBlueprintFunctionLibrary.FindCustomDataFragmentFromContext` "/Script/FinalFantasyXI.DamageGameplayContext" _contexthandle))
    (:`Valid`
      _)
    (:`NotValid`
      _))
  (`self.K2_EndAbility`))